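; BP_Enemy is an enemy actor that travels in a straight line toward where the player was when it spawned.
; On BeginPlay it finds the BP_Player actor, stores it as Target, and calls FindDirection to compute a normalized direction to it.
; Tick moves the actor along that fixed direction by Speed scaled with delta time, without sweeping, so it does not home in.
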(event EventBeginPlay
  (bind _returnvalue (Actor|GetActorOfClass "/Game/Blueprints/BP_Player.BP_Player_C"))
  (Variables|Default|SetTarget _returnvalue)
  (CallFunction|FindDirection))

(event Collision|EventActorBeginOverlap
  (params (OtherActor :type Actor%20Object%20Reference)))

(event EventTick
  (params (DeltaSeconds :type Float%20%28single-precision%29))
  (Transformation|SetActorLocation (+ (* (* (Variables|Default|GetDirection) (Variables|Default|GetSpeed)) DeltaSeconds) (Transformation|GetActorLocation)) false false))

(fn ConstructionScript)

(fn FindDirection
  (Variables|Default|SetDirection (Math|Vector|Normalize (- (Transformation|GetActorLocation (Variables|Default|GetTarget)) (Transformation|GetActorLocation)))))