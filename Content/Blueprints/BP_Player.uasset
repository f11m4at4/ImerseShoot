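; BP_Player is the player-controlled actor that moves in the Y/Z plane and shoots bullets.
; Horizontal and Vertical axis inputs set Direction, and each calls Movement, so it runs from both events.
; Movement applies P = P0 + vt using normalized Direction, Speed and delta time, setting location without sweeping for collisions.
; Pressing Fire spawns a BP_Bullet at the actor's transform, regardless of collisions.
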(event EventTick
  (params (DeltaSeconds :type Float%20%28single-precision%29)))

(event Input|ActionEvents|InputActionFire
  (params (Key :type Key%20Structure :default "None"))
  (:Pressed
    (Game|SpawnActorfromClass "/Game/Blueprints/BP_Bullet.BP_Bullet_C" (Transformation|GetActorTransform) "AlwaysSpawn" 0 0)))

(event Input|AxisEvents|InputAxisHorizontal
  (params (AxisValue :type Float%20%28single-precision%29))
  (Variables|Default|SetDirection (Math|Vector|MakeVector 0.0 AxisValue (.z (Variables|Default|GetDirection))))
  (CallFunction|Movement 0.0))

(event Input|AxisEvents|InputAxisVertical
  (params (AxisValue :type Float%20%28single-precision%29))
  (Variables|Default|SetDirection (Math|Vector|MakeVector 0.0 (.y (Variables|Default|GetDirection)) AxisValue))
  (CallFunction|Movement 0.0))

(fn ConstructionScript)

(fn Movement
  (params (B :type Float%20%28single-precision%29))
  ;[1 1 1] P
  (Transformation|SetActorLocation (+ (Transformation|GetActorLocation) (* (* (Math|Vector|Normalize (Variables|Default|GetDirection)) (Variables|Default|GetSpeed)) (Utilities|Time|GetWorldDeltaSeconds))) false false))